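; BP_CreakingFloor is a trigger actor that plays a creaking floor sound when the player steps into its Box.
; BeginPlay creates a persistent, non-spatial 2D audio component from CreakingFloor_Cue and passes it to AddAnAudio.
; On Box overlap, it compares the other actor's class to the player pawn's class and, on a match, plays the sound from the start.
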(event `self.ReceiveBeginPlay`
  ;[1 1 1] Creaking floor Audio
  (bind _returnvalue (`GameplayStatics.CreateSound2D` "/Game/SFX/CreakingFloor_Cue.CreakingFloor_Cue" 1.0 1.0 0.0 null false false))
  (bind _output_get (set `self.CreakingFloorAudio` _returnvalue))
  ;[1 1 1] Walk sound effect
  (`/Game/Blueprints/Widgets/MenuLibrary.AddAnAudio` true null _output_get))

(event `self.Box.OnComponentBeginOverlap`
  (params (OverlappedComponent :type "PrimitiveComponent Object Reference") (OtherActor :type "Actor Object Reference") (OtherComp :type "PrimitiveComponent Object Reference") (OtherBodyIndex :type Integer) (bFromSweep :type Boolean) (SweepResult :type "HitResult Structure (by ref)"))
  ;[1 1 1] If player
  (if (== (`GameplayStatics.GetObjectClass` OtherActor) (`GameplayStatics.GetObjectClass` (`GameplayStatics.GetPlayerPawn` 0)))
    ;[1 1 1] Play audio
    (`AudioComponent.Play` (`self.CreakingFloorAudio`) 0.0)))

(fn `UserConstructionScript`)