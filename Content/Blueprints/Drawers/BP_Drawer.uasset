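; BP_Drawer is an interactable drawer Blueprint that supplies sound feedback for opening and closing.
; OnOpen and OnClose start their cues through Sound.StartSound and pass the resulting audio to AddAnAudio.
; Lock, unlock and interaction events are empty.
; Locked-door and unlocking sound chains, including a two-step SoundUnlockToOpen call, remain disconnected, as does a 2D opening sound.
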(event `self.OnLock`
  ;[1 1 1] Gestion du son
)

(event `self.OnUnlock`
  ;[1 1 1] Gestion du son
)

(event `self.OnOpen`
  ;[1 1 1] Gestion du son
  (bind _outaudio (`SoundManager.StartSound` (`self.Sound`) "/Game/SFX/opening_drawer_Cue.opening_drawer_Cue"))
  ;[1 1 1] Sound effects
  (`/Game/Blueprints/Widgets/MenuLibrary.AddAnAudio` true null _outaudio))

(event `self.OnClose`
  ;[1 1 1] Gestion du son
  (bind _outaudio (`SoundManager.StartSound` (`self.Sound`) "/Game/SFX/close_drawer_Cue.close_drawer_Cue"))
  ;[1 1 1] Sound effects
  (`/Game/Blueprints/Widgets/MenuLibrary.AddAnAudio` true null _outaudio))

(event `self.OnInteraction_BP`)

(fn `UserConstructionScript`)