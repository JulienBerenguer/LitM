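; BP_InputsForcer registers the game's input mappings from code on BeginPlay, covering Interact, OpenPuzzle, movement and camera look.
; A sequence feeds two wrapper macros, AddAction and AddAxis, which add keyboard, mouse and gamepad bindings to Input Settings.
; Movement uses an AZERTY ZQSD layout and the gamepad right stick, leaving the left stick for camera rates.
; Only MouseY LookUp gets a removal call before being re-added with negative scale.
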(event `self.ReceiveBeginPlay`
  (`|ExecutionSequence`
    (:`then_0`
      (`self.AddAction` "Interact" "E"
        (:`Out`
          (`self.AddAction` "Interact" "LeftMouseButton"
            (:`Out`
              (`self.AddAction` "Interact" "Gamepad_RightTrigger"
                (:`Out`
                  (`self.AddAction` "Interact" "Gamepad_FaceButton_Bottom"))))))))
    (:`then_1`
      (`self.AddAction` "OpenPuzzle" "F"
        (:`Out`
          (`self.AddAction` "OpenPuzzle" "Gamepad_Special_Left"))))
    (:`then_2`
      (`self.AddAxis` "MoveForward" 1.0 "Z"
        (:`Out`
          (`self.AddAxis` "MoveForward" -1.0 "S"
            (:`Out`
              (`self.AddAxis` "MoveForward" 1.0 "Gamepad_RightY"))))))
    (:`then_3`
      (`self.AddAxis` "MoveRight" 1.0 "D"
        (:`Out`
          (`self.AddAxis` "MoveRight" -1.0 "Q"
            (:`Out`
              (`self.AddAxis` "MoveRight" 1.0 "Gamepad_RightX"))))))
    (:`then_4`
      (`self.AddAxis` "Turn" 1.0 "MouseX"
        (:`Out`
          (`self.AddAxis` "TurnRate" -1.0 "Gamepad_LeftX"))))
    (:`then_5`
      (`InputSettings.RemoveAxisMapping` (`InputSettings.GetInputSettings`) (make `InputAxisKeyMapping` "LookUp" 1.0 "MouseY") true)
      (`self.AddAxis` "LookUp" -1.0 "MouseY"
        (:`Out`
          (`self.AddAxis` "LookUpRate" -1.0 "Gamepad_LeftY"))))))

(fn `UserConstructionScript`)