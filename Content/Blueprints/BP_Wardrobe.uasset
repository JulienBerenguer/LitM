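; BP_Wardrobe is an interactable wardrobe built from Furniture child actors, including its doors, that act together.
; On BeginPlay it nearly mutes the right door's audio so only one door is heard, then passes its KeyRef to every child Furniture and calls Init.
; Interacting with the wardrobe forwards OnInteraction to all child Furniture, so both doors respond at once.
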(event `self.ReceiveBeginPlay`
  ;[1 1 1] Garde le son que d'une seule porte
  (bind _asfurniture (cast `Furniture` (`ChildActorComponent.ChildActor` (`self.BP_WardrobeDoorR`))))
  (set `Furniture.AudioVolumeMultiplier` 0.001 _asfurniture)
  ;[1 1 1] Assigne la clé aux deux portes
  (for _array_element (`self.GetAllChildActors` true)
    (bind _asfurniture_2 (cast `Furniture` _array_element))
    (set `Furniture.KeyRef` (`self.KeyRef`) _asfurniture_2)
    (`self.Init` _asfurniture_2)))

(event `self.OnInteraction_BP`
  ;[1 1 1] OnInteraction sur les portes également
  (for _array_element (`self.GetAllChildActors` true)
    (bind _asfurniture (cast `Furniture` _array_element))
    (`self.OnInteraction` _asfurniture)))

(fn `UserConstructionScript`)