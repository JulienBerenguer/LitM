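; BP_Key is an interactable key actor that shows its name in floating text when looked at.
; Interaction creates and plays a 2D pickup cue registered through AddAnAudio, while a look event sets the name text and calls NotLookAtActor after a short delay.
; OnDestroy disables collision and hides the components rather than destroying the actor.
; Tick rotates the text to face the player pawn.
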(event `self.OnInteraction_BP`
  ;[1 1 1] Sound
  (bind _returnvalue (`GameplayStatics.CreateSound2D` "/Game/SFX/key_01_Cue.key_01_Cue" 1.0 1.0 0.0 null))
  (`/Game/Blueprints/Widgets/MenuLibrary.AddAnAudio` true null _returnvalue)
  (`AudioComponent.Play` _returnvalue 0.0))

(event `self.OnLookAtActor`
  ;[1 1 1] LookAt -> Show Key Name
  (`TextRenderComponent.K2_SetText` (`self.TextRender1`) (`KismetTextLibrary.Conv_StringToText` (`self.Name`)))
  ;;[1 1 1] Don't look trigger
  (`KismetSystemLibrary.Delay` 2.0)
  (`self.NotLookAtActor`))

(event `self.OnNotLookAtActor`
  ;[1 1 1] NotLookAt -> Hide Key Name
  (`TextRenderComponent.K2_SetText` (`self.TextRender1`) ""))

(event `self.OnDestroy`
  ;[1 1 1] Is Used
  (`PrimitiveComponent.SetCollisionEnabled` (`self.Capsule`) "NoCollision")
  (`PrimitiveComponent.SetCollisionEnabled` (`self.ObjectMesh`) "NoCollision")
  (`SceneComponent.SetHiddenInGame` (`self.RootScene`) true true))

(event `self.ReceiveTick`
  (params (DeltaSeconds :type "Float (single-precision)"))
  (bind _textrender1 (`self.TextRender1`))
  ;[1 1 1] Event tick : Look at
  (`SceneComponent.K2_SetWorldRotation` _textrender1 (`KismetMathLibrary.FindLookAtRotation` (`SceneComponent.K2_GetComponentLocation` _textrender1) (`self.K2_GetActorLocation` (`GameplayStatics.GetPlayerPawn` 0))) false false))

(fn `UserConstructionScript`)