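; Interactable tape recorder that plays an audio recording and shows the logbook tutorial on interaction.
; Sound start plays an activation cue, then starts the recording through Sound and plays a deactivation cue when it finishes.
; Both cues and voice are registered via AddAnAudio for volume management.
; Destruction hides the actor and disables mesh collision, with a temporary flag to trigger it at BeginPlay.
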(event `self.ReceiveBeginPlay`
  ;[1 1 1] Temporaire pour les faire disparaître de la scène
  (if (`self.DestroyItAtBeginPlay`)
    (`self.DestroyIt` true)))

(event `self.OnDestroy`
  ;[1 1 1] Is Used
  (`PrimitiveComponent.SetCollisionEnabled` (`self.ObjectMesh`) "NoCollision")
  (`SceneComponent.SetHiddenInGame` (`self.RootScene`) true true))

(event `self.OnInteraction_BP`
  ;[1 1 1] Logbook Tuto (DoOnce)
  (`/Game/Blueprints/Tuto/TutoLibrary.ShowTuto` "/Game/Blueprints/Tuto/WBP_TutoLogbook.WBP_TutoLogbook_C"))

(event `self.OnSoundStart`
  ;[1 1 1] Audio
  ;;[1 1 1] Start audio
  ;;;[1 1 1] Tape activation
  (bind _returnvalue (`GameplayStatics.CreateSound2D` "/Game/SFX/Activate_Tape_Cue.Activate_Tape_Cue" 1.0 1.0 0.0 null))
  (`/Game/Blueprints/Widgets/MenuLibrary.AddAnAudio` true null _returnvalue)
  (`AudioComponent.Play` _returnvalue 0.0)
  ;;;[1 1 1] Start Audio
  (bind _outaudio (`SoundManager.StartSound` (`self.Sound`) (`self.Audio`)))
  ;;;[1 1 1] Volume management
  (`/Game/Blueprints/Widgets/MenuLibrary.AddAnAudio` true _outaudio)
  ;;;[1 1 1] Audio finished
  (add `AudioComponent.OnAudioFinished` _outaudio (delegate `OnAudioFinished_Event_0`)))

(event `OnAudioFinished_Event_0`
  ;[1 1 1] Audio
  ;;[1 1 1] Start audio
  ;;;[1 1 1] Audio finished
  ;;;;[1 1 1] Tape deactivation
  (bind _returnvalue (`GameplayStatics.CreateSound2D` "/Game/SFX/Deactivate_tape_Cue.Deactivate_tape_Cue" 1.0 1.0 0.0 null))
  (`/Game/Blueprints/Widgets/MenuLibrary.AddAnAudio` true null _returnvalue)
  (`AudioComponent.Play` _returnvalue 0.0))

(event `self.OnSoundPlay`
  ;[1 1 1] Audio
  ;;[1 1 1] Play audio (unused now)
  ;;;[1 1 1] Play Audio
  (`SoundManager.PlaySound` (`self.Sound`)))

(event `self.OnSoundStop`
  ;[1 1 1] Audio
  ;;[1 1 1] Stop audio
  ;;;[1 1 1] Stop Audio
  (`SoundManager.StopSound` (`self.Sound`)))

(event `self.OnSoundAnotherTapeStop`
  ;[1 1 1] Audio
  ;;[1 1 1] Stop all other tape audio when a new tape start
)

(fn `UserConstructionScript`)