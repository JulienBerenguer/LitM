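; Temporary pawn that drives the logbook menu in place of the player character, matching its FOV and creating WBP_Logbook on Init.
; Movement, D-pad, shoulder and Interact inputs forward to the widget, with axes gated by a threshold and a Tick-driven repeat cooldown.
; OpenPuzzle or Return removes the widget, repossesses the character with this camera's rotation and destroys the pawn.
; SetOutro advances to the puzzle panel and locks all input.
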(event `self.ReceiveBeginPlay`)

(event `InputAction|OpenPuzzle`
  (params (Key :type "Key Structure"))
  (bind _returnvalue (`GameplayStatics.GetPlayerController` 0))
  (bind _playercharacter (`self.PlayerCharacter`))
  (:`Pressed`
    (`self.CanUseInputs` :!label _label
      (:`True`
        ;[1 1 1] Save camera rotation
        (`/Engine/EditorBlueprintResources/StandardMacros.IsValid` _playercharacter
          (:`Is Valid`
            (set `self.CameraTransform` (`SceneComponent.K2_GetComponentRotation` (`self.Camera`)))
            ;[1 1 1] Possess the character + undo init
            (`Controller.Possess` _returnvalue _playercharacter)
            (`Widget.RemoveFromParent` (`self.Widget`))
            (`WidgetBlueprintLibrary.SetInputMode_GameOnly` _returnvalue)
            (set `PlayerController.bShowMouseCursor` false _returnvalue)
            ;[1 1 1] Set camera rotation
            (`Controller.SetControlRotation` _returnvalue (`self.CameraTransform`))
            ;[1 1 1] If sheet opened
            (`LitMCharacter.CloseSheet` (`self.PlayerCharacter`))
            ;[1 1 1] Destroy pawn
            (`self.K2_DestroyActor` self))
          (:`Is Not Valid`
            (`KismetSystemLibrary.PrintString` "ERROR BP_MenuNavigatorPawn : PlayerCharacter not set !")))))))

(event `InputAction|Return`
  (params (Key :type "Key Structure"))
  (:`Pressed`
    (goto _label)))

(event `Init`
  (bind _returnvalue (`GameplayStatics.GetPlayerController` 0))
  (bind _playercharacter (`self.PlayerCharacter`))
  ;[1 1 1] Set FOV
  (`/Engine/EditorBlueprintResources/StandardMacros.IsValid` _playercharacter
    (:`Is Valid`
      (`CameraComponent.SetFieldOfView` (`self.Camera`) (`CameraComponent.FieldOfView` (`LitMCharacter.FirstPersonCameraComponent` _playercharacter)))
      ;[1 1 1] Create widget
      (bind _returnvalue_2 (`|CreateWidget` "/Game/Blueprints/Logbook/WBP_Logbook.WBP_Logbook_C"))
      (bind _output_get (set `self.Widget` _returnvalue_2))
      (`UserWidget.AddToViewport` _output_get 0)
      (`WidgetBlueprintLibrary.SetInputMode_GameAndUIEx` _returnvalue _output_get "LockAlways" false)
      (set `PlayerController.bShowMouseCursor` true _returnvalue))
    (:`Is Not Valid`
      (`KismetSystemLibrary.PrintString` "ERROR BP_MenuNavigatorPawn : PlayerCharacter not set !"))))

(event `InputAxis|MoveForward` :paused true
  (params (AxisValue :type "Float (single-precision)"))
  (bind _widget (`self.Widget`))
  ;[1 1 1] Move
  (set `self.TempAxisForward` AxisValue)
  (`self.CanUseInputs` :!label _label_2
    (:`True`
      (`self.Move` (`self.TempAxisForward`)
        (:`Positive`
          (`/Game/Blueprints/Logbook/WBP_Logbook.MoveUp` _widget))
        (:`Negative`
          (`/Game/Blueprints/Logbook/WBP_Logbook.MoveDown` _widget))))))

(event `InputAxis|DpadForward`
  (params (AxisValue :type "Float (single-precision)"))
  ;[1 1 1] Move
  (set `self.TempAxisForward` AxisValue)
  (goto _label_2))

(event `InputAxis|MoveRight` :paused true
  (params (AxisValue :type "Float (single-precision)"))
  (bind _widget (`self.Widget`))
  ;[1 1 1] Move
  (set `self.TempAxisRight` AxisValue)
  (`self.CanUseInputs` :!label _label_3
    (:`True`
      (`self.Move` (`self.TempAxisRight`)
        (:`Positive`
          (`/Game/Blueprints/Logbook/WBP_Logbook.MoveRight` _widget))
        (:`Negative`
          (`/Game/Blueprints/Logbook/WBP_Logbook.MoveLeft` _widget))))))

(event `InputAxis|DpadRight`
  (params (AxisValue :type "Float (single-precision)"))
  ;[1 1 1] Move
  (set `self.TempAxisRight` AxisValue)
  (goto _label_3))

(event `InputAxis|GamepadShoulders`
  (params (AxisValue :type "Float (single-precision)"))
  (bind _widget (`self.Widget`))
  ;[1 1 1] Shoulders (gamepad)
  (`self.CanUseInputs`
    (:`True`
      (`self.Move` AxisValue
        (:`Positive`
          (`/Game/Blueprints/Logbook/WBP_Logbook.ShoulderRight` _widget))
        (:`Negative`
          (`/Game/Blueprints/Logbook/WBP_Logbook.ShoulderLeft` _widget))))))

(event `InputAction|Interact`
  (params (Key :type "Key Structure"))
  ;[1 1 1] Button Validation
  (:`Pressed`
    (`self.CanUseInputs`
      (:`True`
        (`/Game/Blueprints/Logbook/WBP_Logbook.Validation` (`self.Widget`))))))

(event `self.ReceiveTick`
  (params (DeltaSeconds :type "Float (single-precision)"))
  ;[1 1 1] Move time
  (if (> (`self.TimeMove`) 0.0)
    (set `self.TimeMove` (- (`self.TimeMove`) DeltaSeconds))
    (else
      (set `self.TimeMove` 0.0))))

(fn `SetOutro`
  (bind _widget (`self.Widget`))
  ;[1 1 1] Go to puzzle panel
  (`/Game/Blueprints/Logbook/WBP_Logbook.ButtonNavigation` _widget "Next")
  ;[1 1 1] Disable Left / Right Logbook Buttons
  (`/Game/Blueprints/Logbook/WBP_Logbook.DisableButtons` _widget)
  ;[1 1 1] Cannot use inputs anymore
  (set `self.PlayerCanUseInputs` false)
  ;[1 1 1] Hide mouse cursor
  (set `PlayerController.bShowMouseCursor` false (`GameplayStatics.GetPlayerController` 0))
  (return))

(fn `UserConstructionScript`)