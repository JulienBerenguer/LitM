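; Door Blueprint that handles lock, unlock, open and close sound feedback and shows a name label when looked at.
; Each state event starts a cue and registers it via AddAnAudio; unlocking also calls SoundUnlockToOpen for two-step opening.
; Both text renders show the door's Name, else the referenced KeyObject's (or child's) name while locked or if ShowNameAfterUnlock is set.
; After a delay it calls NotLookAtActor; OnNotLookatActor clears the text.
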(event `self.OnLock`
  ;[1 1 1] Gestion du son
  (bind _outaudio (`SoundManager.StartSound` (`self.Sound`) "/Game/SFX/locked_door_01_Cue.locked_door_01_Cue"))
  ;[1 1 1] Sound effects
  (`/Game/Blueprints/Widgets/MenuLibrary.AddAnAudio` true null _outaudio))

(event `self.OnUnlock`
  ;[1 1 1] Gestion du son
  (bind _outaudio (`SoundManager.StartSound` (`self.Sound`) "/Game/SFX/unlocking_Cue.unlocking_Cue"))
  ;[1 1 1] Sound effects
  (`/Game/Blueprints/Widgets/MenuLibrary.AddAnAudio` true null _outaudio)
  ;[1 1 1] Ouverture en deux temps
  (`self.SoundUnlockToOpen`))

(event `self.OnOpen`
  ;[1 1 1] Gestion du son
  (bind _outaudio (`SoundManager.StartSound` (`self.Sound`) "/Game/SFX/opening-door_Cue.opening-door_Cue"))
  ;[1 1 1] Sound effects
  (`/Game/Blueprints/Widgets/MenuLibrary.AddAnAudio` true null _outaudio))

(event `self.OnClose`
  ;[1 1 1] Gestion du son
  (bind _outaudio (`SoundManager.StartSound` (`self.Sound`) "/Game/SFX/closing_door_Cue.closing_door_Cue"))
  ;[1 1 1] Sound effects
  (`/Game/Blueprints/Widgets/MenuLibrary.AddAnAudio` true null _outaudio))

(event `self.OnLookAtActor`
  (bind _keyref (`self.KeyRef`))
  ;[1 1 1] LookAt -> Show Key Name
  (`/Engine/EditorBlueprintResources/StandardMacros.IsValid` _keyref
    (:`Is Valid`
      ;;[1 1 1] Door name empty ?
      (if (`KismetStringLibrary.NotEqual_StrStr` (`self.Name`))
        ;;[1 1 1] No key path Or key path with door name not empty
        (set `self.KeyName` (`self.Name`) :!label _label)
        ;;[1 1 1] Set name on text render
        (`TextRenderComponent.K2_SetText` (`self.TextRender1`) (`KismetTextLibrary.Conv_StringToText` (`self.KeyName`)) :!label _label_2)
        (`TextRenderComponent.K2_SetText` (`self.TextRender2`) (`KismetTextLibrary.Conv_StringToText` (`self.KeyName`)))
        ;[1 1 1] Don't look trigger
        (`KismetSystemLibrary.Delay` 2.0 :!label _label_3)
        (`self.NotLookAtActor`)
        (else
          ;;[1 1 1] Show key name even if unlocked ?
          (if (`self.ShowNameAfterUnlock`)
            _
            (elif (`self.IsLocked`)
              _
              (else
                (goto _label_3))))
          ;;[1 1 1] Key path with door name empty
          (bind _askey_object (cast `KeyObject` _keyref)
            (:`then`
              (set `self.KeyName` (`Item.Name` _askey_object))
              (goto _label_2))
            (:`CastFailed`
              (for _array_element (`self.GetAllChildActors` _keyref true)
                (bind _askey_object_2 (cast `KeyObject` _array_element))
                (set `self.KeyName` (`Item.Name` _askey_object_2))
                (goto _label_2)))))))
    (:`Is Not Valid`
      (goto _label))))

(event `self.OnNotLookAtActor`
  ;[1 1 1] NotLookAt -> Hide Key Name
  (`TextRenderComponent.K2_SetText` (`self.TextRender1`) "")
  (`TextRenderComponent.K2_SetText` (`self.TextRender2`) ""))

(fn `UserConstructionScript`)