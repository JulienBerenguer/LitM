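; BP_Obstacle is a destructible obstacle actor that swaps between two meshes when destroyed.
; At BeginPlay it hides ObjectMesh1 and disables its collision, keeping it in reserve as the destroyed-state mesh.
; OnDestroy runs once, playing a 2D falling sound registered through AddAnAudio, then inverts visibility and collision so ObjectMesh1 replaces ObjectMesh without removing the actor.
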(event `self.ReceiveBeginPlay`
  (bind _objectmesh1 (`self.ObjectMesh1`))
  (`SceneComponent.SetVisibility` _objectmesh1 false true)
  (`PrimitiveComponent.SetCollisionEnabled` _objectmesh1 "NoCollision"))

(event `self.OnDestroy`
  (bind _objectmesh1 (`self.ObjectMesh1`))
  (bind _objectmesh (`self.ObjectMesh`))
  ;[1 1 1] Falling sound
  (`/Engine/EditorBlueprintResources/StandardMacros.DoOnce` false
    (:`Completed`
      (bind _returnvalue (`GameplayStatics.SpawnSound2D` (`self.DestroySound`) 1.0 1.0 0.0 null))
      (`/Game/Blueprints/Widgets/MenuLibrary.AddAnAudio` true null _returnvalue)
      (`AudioComponent.Play` _returnvalue 0.0)
      ;[1 1 1] Invert mesh show
      (`SceneComponent.SetVisibility` _objectmesh1 true true)
      (`PrimitiveComponent.SetCollisionEnabled` _objectmesh1 "QueryAndPhysics")
      (`SceneComponent.SetVisibility` _objectmesh false true)
      (`PrimitiveComponent.SetCollisionEnabled` _objectmesh "NoCollision"))))

(fn `UserConstructionScript`)