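; BP_WardrobeDoor is a wardrobe door Blueprint that supplies the sounds for lock, unlock, open and close events.
; Each event starts its own cue through Sound.StartSound, and lock, unlock and close pass the result to AddAnAudio.
; Unlock also calls SoundUnlockToOpen for a two-stage opening.
; The open event starts its cue, but its AddAnAudio call is disconnected and never runs.
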(event `self.OnLock`
  ;[1 1 1] Gestion du son
  (bind _outaudio (`SoundManager.StartSound` (`self.Sound`) "/Game/SFX/locked_door_01_Cue.locked_door_01_Cue"))
  ;[1 1 1] Sound effects
  (`/Game/Blueprints/Widgets/MenuLibrary.AddAnAudio` true null _outaudio))

(event `self.OnUnlock`
  ;[1 1 1] Gestion du son
  (bind _outaudio (`SoundManager.StartSound` (`self.Sound`) "/Game/SFX/unlocking_Cue.unlocking_Cue"))
  ;[1 1 1] Sound effects
  (`/Game/Blueprints/Widgets/MenuLibrary.AddAnAudio` true null _outaudio)
  ;[1 1 1] Ouverture en deux temps
  (`self.SoundUnlockToOpen`))

(event `self.OnOpen`
  ;[1 1 1] Gestion du son
  (bind _outaudio (`SoundManager.StartSound` (`self.Sound`) "/Game/SFX/opening-door_Cue.opening-door_Cue")))

(event `self.OnClose`
  ;[1 1 1] Gestion du son
  (bind _outaudio (`SoundManager.StartSound` (`self.Sound`) "/Game/SFX/closing_door_Cue.closing_door_Cue"))
  ;[1 1 1] Sound effects
  (`/Game/Blueprints/Widgets/MenuLibrary.AddAnAudio` true null _outaudio))

(fn `UserConstructionScript`)